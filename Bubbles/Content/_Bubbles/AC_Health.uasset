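; Health component that tracks hit points, starting at the maximum when play begins.
; TakeDamage prints a debug message and subtracts damage, clamped between zero and the maximum.
; At zero health it opens LVL_Main after a short delay, with no separate death handling.
; Non-lethal hits instead raise the global "BubblesDestroyed" parameter by a small random amount.
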(event `self.ReceiveBeginPlay`
  (set `self.CurrentHealthpoints` (`self.MaxHealthPoints`)))

(event `TakeDamage`
  (params (amount :type Integer))
  (`KismetSystemLibrary.PrintString` "Hello")
  (bind _output_get (set `self.CurrentHealthpoints` (`KismetMathLibrary.Clamp` (- (`self.CurrentHealthpoints`) amount) 0 (`self.MaxHealthPoints`))))
  (if (<= _output_get 0)
    (`KismetSystemLibrary.Delay` 0.5)
    (`GameplayStatics.OpenLevel` "LVL_Main")
    (else
      (bind _returnvalue (`FMODBlueprintStatics.GetGlobalParameterByName` "BubblesDestroyed"))
      (`FMODBlueprintStatics.SetGlobalParameterByName` "BubblesDestroyed" (+ _returnvalue (`KismetMathLibrary.Conv_IntToDouble` (+ (`KismetMathLibrary.RandomInteger` 3) 1)))))))